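; Crafting component that holds a fixed number of active recipe slots and shows their craft panel on the player's HUD.
; AddRecipe fills slots with hard-coded handling for one or two (flagged as unsafe), then rebuilds WBP_CraftPanel through PC_Configurator's HUD canvas.
; CreateNewItem spawns the slot's crafted actor near the player's mesh, clears the slot and removes the panel.
; GatherItems only increments a counter; its completion branch is empty.
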(event `self.ReceiveBeginPlay`
  (`self.PrepareRecipeWidget`))

(fn `AddRecipe`
  (params (Recipe :type "/Game/CraftingSystem/Recipes/SRecipe Structure"))
  (if (== (`self.NumberOfRecipeSlots`) 1)
    (bind _craft_panel (`self.Craft Panel`)
      (:`then`
        (`Widget.RemoveFromParent` _craft_panel))
      (:`else`
        _))
    (`KismetArrayLibrary.Array_Set` (`self.RecipeSlots`) 0 (`local.Recipe`)) ; Это помешает в дальнейшем добавлению\nрецептов, которые можно отобразить за раз!
    (`self.CreateCraftPanel` :!label _label)
    (set `self.NumberOfNeededIngredients` (`.QuantityOfIngredients_13_CB4F806B462C9D70D0FB559533B32246` (break `/Game/CraftingSystem/Recipes/SRecipe` (`local.Recipe`))))
    (elif (== (`self.NumberOfRecipeSlots`) 2)
      (`self.Craft Panel`
        (:`then`
          (if (`KismetMathLibrary.Conv_IntToBool` (`.QuantityOfIngredients_13_CB4F806B462C9D70D0FB559533B32246` (break `/Game/CraftingSystem/Recipes/SRecipe` (`|GetArrayItem` (`self.RecipeSlots`) 1))))
            (`Widget.RemoveFromParent` (`self.Craft Panel`)))
          (`KismetArrayLibrary.Array_Set` (`self.RecipeSlots`) 1 (`local.Recipe`))
          (goto _label))
        (:`else`
          (`KismetArrayLibrary.Array_Set` (`self.RecipeSlots`) 0 (`local.Recipe`))
          (goto _label))))))

(fn `CreateCraftPanel`
  (bind _returnvalue (`|CreateWidget` "/Game/CraftingSystem/CraftUI/WBP_CraftPanel.WBP_CraftPanel_C" null self))
  (set `self.Craft Panel` _returnvalue)
  (bind _aspc_configurator (cast `/Game/GameBase/PC_Configurator` (`GameplayStatics.GetPlayerController` 0)))
  (bind _returnvalue_2 (`CanvasPanel.AddChildToCanvas` (`/Game/InventorySystem/InventoryUI/HUD.HudCanvas` (`/Game/GameBase/PC_Configurator.HudWidget` _aspc_configurator)) (`self.Craft Panel`)))
  (`CanvasPanelSlot.SetAutoSize` _returnvalue_2 true)
  (`CanvasPanelSlot.SetAlignment` _returnvalue_2 (0.0 0.0))
  (`CanvasPanelSlot.SetAnchors` :`self` _returnvalue_2)
  (return))

(fn `CreateNewItem`
  (params (SlotIndex :type Integer))
  (bind (_output_image _output_ingredient _output_craftedthing) (break `/Game/CraftingSystem/Recipes/SRecipe` (`|GetArrayItem` (`self.RecipeSlots`) SlotIndex)))
  (`|SpawnActorFromClass` _output_craftedthing (`KismetMathLibrary.Conv_VectorToTransform` (+ (`SceneComponent.GetSocketLocation` (`Character.Mesh` (`GameplayStatics.GetPlayerCharacter` 0)) "None") (0.0 100.0 0.0))) "Undefined" "OverrideRootScale" null null)
  (`KismetArrayLibrary.Array_Set` (`self.RecipeSlots`) (`local.SlotIndex`))
  (`Widget.RemoveFromParent` (`self.Craft Panel`)))

(fn `Gather Items`
  (params (RecipeIndex :type Integer) (TypeOfItem :type "/Game/InventorySystem/Item/BP_Item Class Reference"))
  (bind _output_get (set `self.GatheredCompletely` (+ (`self.GatheredCompletely`) 1)))
  (if (== _output_get (`self.NumberOfNeededIngredients`))
    _))

(fn `PrepareRecipeWidget`
  ;[1 1 1] Устанавливаем количество рецептов, которое можно взять одновременно
  (`KismetArrayLibrary.Array_Resize` (`self.RecipeSlots`) (`self.NumberOfRecipeSlots`)))