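; BP_Pensilcase is an interactable pencil case that acts as a container through its InventoryComponent.
; On Interact, it reads the first slot of the interacter's InventoryComponent.
; An empty slot toggles the pencil case's inventory, while a filled one is passed to its AddToInventory with a debug "Hello" print.
; The graph itself never removes that item from the interacter.
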(event `/Game/InventorySystem/Interact_Interface.Interact`
  (params (Interacter :type "Actor Object Reference"))
  (bind _output (`|GetArrayItem` (`/Game/InventorySystem/InventoryComponent.Inventory` (`self.GetComponentByClass` Interacter "/Game/InventorySystem/InventoryComponent.InventoryComponent_C"))))
  (if (== (`.Quantity_5_0C99093F40D6DA4DF3C0F8A2D7068DCC` (break `/Game/InventorySystem/SlotStructure` _output)) 0)
    (`/Game/InventorySystem/InventoryComponent.ToggleInventory` (`self.InventoryComponent`))
    (else
      (`/Game/InventorySystem/InventoryComponent.AddToInventory` (`self.InventoryComponent`) _output)
      (`KismetSystemLibrary.PrintString` "Hello"))))

(fn `UserConstructionScript`)