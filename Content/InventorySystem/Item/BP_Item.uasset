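; BP_Item is a pickup actor for the inventory system, carrying an ItemStructure that describes the item.
; On Interact, it adds one of itself to the interacter's InventoryComponent and destroys itself only if that succeeds.
; UseItem is a stub that always returns true.
; RotateMe and RotateMe2 step the relative pitch in opposite directions from the current world rotation; RotateMe also zeroes roll.
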(event `/Game/InventorySystem/Interact_Interface.Interact`
  (params (Interacter :type "Actor Object Reference"))
  (bind _success (`/Game/InventorySystem/InventoryComponent.AddToInventory` (`self.GetComponentByClass` Interacter "/Game/InventorySystem/InventoryComponent.InventoryComponent_C") (make `/Game/InventorySystem/SlotStructure` (`self.ItemStructure`) 1)))
  (if _success
    (`self.K2_DestroyActor`)))

(fn `RotateMe`
  (bind (_returnvalue_roll _returnvalue_pitch _returnvalue_yaw) (`KismetMathLibrary.BreakRotator` (`self.K2_GetActorRotation` self)))
  (`self.K2_SetActorRelativeRotation` (`KismetMathLibrary.MakeRotator` 0.0 (+ _returnvalue_pitch 5.0) _returnvalue_yaw)))

(fn `RotateMe2`
  (bind (_returnvalue_roll _returnvalue_pitch _returnvalue_yaw) (`KismetMathLibrary.BreakRotator` (`self.K2_GetActorRotation` self)))
  (`self.K2_SetActorRelativeRotation` (`KismetMathLibrary.MakeRotator` _returnvalue_roll (+ _returnvalue_pitch -5.0) _returnvalue_yaw)))

(fn `UseItem`
  (returns (Success :type Boolean))
  (return true))

(fn `UserConstructionScript`)