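; BP_Pencilcase is an interactable inventory item that can either be picked up or receive items.
; On Interact, if the interacter's first inventory slot has zero quantity, it adds one of its ItemStructure to that inventory and destroys itself on success.
; Otherwise it adds the contents of that first slot to its own InventoryComponent, without removing them from the interacter.
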(event `/Game/InventorySystem/Interact_Interface.Interact`
  (params (Interacter :type "Actor Object Reference"))
  (bind _returnvalue (`self.GetComponentByClass` Interacter "/Game/InventorySystem/InventoryComponent.InventoryComponent_C"))
  (bind _output (`|GetArrayItem` (`/Game/InventorySystem/InventoryComponent.Inventory` _returnvalue)))
  (if (== (`.Quantity_5_0C99093F40D6DA4DF3C0F8A2D7068DCC` (break `/Game/InventorySystem/SlotStructure` _output)) 0)
    (bind _success (`/Game/InventorySystem/InventoryComponent.AddToInventory` _returnvalue (make `/Game/InventorySystem/SlotStructure` (`self.ItemStructure`) 1)))
    (if _success
      (`self.K2_DestroyActor`))
    (else
      (`/Game/InventorySystem/InventoryComponent.AddToInventory` (`self.InventoryComponent`) _output))))

(fn `UserConstructionScript`)