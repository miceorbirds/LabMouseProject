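; BP_CraftOfLadderComponent is a crafting component that tracks harvested materials and decides whether a ladder can be built.
; HarvestItems counts BP_Item_Pencil pickups up to WantedAmountOfPencils and treats any other item as rubber, setting CanMakeLadder from both.
; The first rubber also runs the pencil check, incrementing an incomplete count, and any later non-pencil item enables crafting regardless of pencil count.
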(fn `HarvestItems`
  (params (ItemInHeap :type "Actor Object Reference"))
  (bind _amountofpencils (`self.AmountOfPencils`))
  (if (== ItemInHeap "/Game/InventorySystem/Item/BP_Item_Pencil.BP_Item_Pencil")
    (if (== (`self.WantedAmountOfPencils`) _amountofpencils) :!label _label
      (if (`self.isRubberThere`)
        (set `self.CanMakeLadder` true :!label _label_2)
        (else
          (set `self.CanMakeLadder` false :!label _label_3)))
      (else
        (set `self.AmountOfPencils` (+ _amountofpencils 1))
        (goto _label_3)))
    (elif (`self.isRubberThere`)
      (goto _label_2)
      (else
        (set `self.isRubberThere` true)
        (goto _label))))
  (return))