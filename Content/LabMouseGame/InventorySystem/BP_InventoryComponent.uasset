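; Inventory component that stores items in a fixed-size slot array and toggles an inventory window on the PC_Configurator HUD canvas.
; BeginPlay sizes the array, and toggling the window also switches input mode and mouse cursor.
; AddToInventory tops up a partial stack of the same item class, recursing with any overflow, or writes to an empty slot.
; It always returns true, with no explicit full-inventory check.
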(event `self.ReceiveBeginPlay`
  (`self.PrepareInventory`))

(fn `AddToInventory`
  (params (ContentToAdd :type "/Game/InventorySystem/SSlot Structure"))
  (returns (Success :type Boolean))
  (if (`.IsStackable_15_56B6C537428752A263B834A426A6D5D8` (break `/Game/InventorySystem/SItem` (break `/Game/InventorySystem/SSlot` ContentToAdd)))
    (bind _stackindex (`self.HasPartialStack` (`local.ContentToAdd`))
      (:`True`
        (`self.AddToStack` (`local.ContentToAdd`) _stackindex))
      (:`False`
        (`self.CreateStack` (`local.ContentToAdd`) :!label _label)))
    (else
      (goto _label)))
  (return true))

(fn `AddToStack`
  (params (SlotStructure :type "/Game/InventorySystem/SSlot Structure") (SlotIndex :type Integer))
  (locals (CurrentStackQuantity :type Integer))
  (bind _inventory (`self.Inventory`))
  (bind _slotindex (`local.SlotIndex`))
  (bind (_slotstructure_itemstructure _slotstructure_quantity) (break `/Game/InventorySystem/SSlot` (`local.SlotStructure`)))
  (bind _slotstructure_itemstructure_2 (break `/Game/InventorySystem/SSlot` (`local.SlotStructure`)))
  (bind (_slotstructure_itemstructure_3 _slotstructure_quantity_2) (break `/Game/InventorySystem/SSlot` (`local.SlotStructure`)))
  (bind (_itemname _itemdescription _thumbnail _class _isstackable _maxstacksize) (break `/Game/InventorySystem/SItem` _slotstructure_itemstructure_2))
  (bind _output (`|GetArrayItem` (`self.Inventory`) SlotIndex))
  (bind (_output_itemstructure _output_quantity) (break `/Game/InventorySystem/SSlot` (`|GetArrayItem` _inventory _slotindex)))
  (bind _output_get (set `local.CurrentStackQuantity` (`.Quantity_5_0C99093F40D6DA4DF3C0F8A2D7068DCC` (break `/Game/InventorySystem/SSlot` _output))))
  (if (> (+ _output_get (`.Quantity_5_0C99093F40D6DA4DF3C0F8A2D7068DCC` (break `/Game/InventorySystem/SSlot` SlotStructure))) (`.MaxStackSize_18_C86CAE394C97FF79A7FA548D6A193ED7` (break `/Game/InventorySystem/SItem` (break `/Game/InventorySystem/SSlot` _output))))
    (`KismetArrayLibrary.Array_Set` (`self.Inventory`) (`local.SlotIndex`) (make `/Game/InventorySystem/SSlot` _slotstructure_itemstructure_2 _maxstacksize))
    (`self.AddToInventory` (make `/Game/InventorySystem/SSlot` _slotstructure_itemstructure_3 (- _slotstructure_quantity_2 (- _maxstacksize (`local.CurrentStackQuantity`)))))
    (else
      (`KismetArrayLibrary.Array_Set` _inventory _slotindex (make `/Game/InventorySystem/SSlot` _output_itemstructure (+ _output_quantity _slotstructure_quantity)))))
  (return))

(fn `CreateStack`
  (params (ContentToAdd :type "/Game/InventorySystem/SSlot Structure"))
  (bind _inventory (`self.Inventory`))
  (`KismetArrayLibrary.Array_Set` _inventory (`KismetArrayLibrary.Array_Find` _inventory (make `/Game/InventorySystem/SSlot` (struct :`ItemName` "NSLOCTEXT(\"[CE05DFC245B94A0F1D3A7DA772DFB9A1]\", \"4BA178D34D0462FB93F23EA55F7DDFB9\", \"None\")" :`ItemDescription` "NSLOCTEXT(\"[CE05DFC245B94A0F1D3A7DA772DFB9A1]\", \"997A96EE4C3972154CF50282AF546982\", \"None\")" :`IsStackable` true :`MaxStackSize` 10 :`IsConsumable` true))) ContentToAdd))

(fn `PrepareInventory`
  (`KismetArrayLibrary.Array_Resize` (`self.Inventory`) (`self.NumberOfSlots`)))

(fn `ToggleInventory`
  (bind _returnvalue (`GameplayStatics.GetPlayerController` 0))
  (bind _returnvalue_2 (`GameplayStatics.GetPlayerController` 0))
  (`self.InventoryWindow`
    (:`then`
      ;[1 1 1] Close Inventory Window
      (`Widget.RemoveFromParent` (`self.InventoryWindow`))
      (set `self.InventoryWindow` null)
      (`WidgetBlueprintLibrary.SetInputMode_GameOnly` _returnvalue_2)
      (set `PlayerController.bShowMouseCursor` false _returnvalue_2))
    (:`else`
      ;[1 1 1] Open Inventory Window
      (bind _returnvalue_3 (`|CreateWidget` "/Game/InventorySystem/InventoryUI/WBP_InventoryWindow.WBP_InventoryWindow_C" null self))
      (set `self.InventoryWindow` _returnvalue_3)
      (bind _aspc_configurator (cast `/Game/GameBase/PC_Configurator` (`GameplayStatics.GetPlayerController` 0)))
      (bind _returnvalue_4 (`CanvasPanel.AddChildToCanvas` (`/Game/InventorySystem/InventoryUI/WBP_HUD.HudCanvas` (`/Game/GameBase/PC_Configurator.HudWidget` _aspc_configurator)) (`self.InventoryWindow`)))
      (`CanvasPanelSlot.SetAutoSize` _returnvalue_4 true)
      (`CanvasPanelSlot.SetAlignment` _returnvalue_4 (0.5 0.5))
      (`CanvasPanelSlot.SetAnchors` _returnvalue_4 (make `Anchors` (0.5 0.5) (0.5 0.5)))
      (`CanvasPanelSlot.SetPosition` _returnvalue_4 (`self.Position`))
      (`WidgetBlueprintLibrary.SetInputMode_UIOnlyEx` _returnvalue (`self.InventoryWindow`) "LockAlways")
      (set `PlayerController.bShowMouseCursor` true _returnvalue))))